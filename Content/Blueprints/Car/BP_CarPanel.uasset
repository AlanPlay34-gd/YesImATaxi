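; Interactive car dashboard with a mouse-steered wheel, rear-view mirror, temperature widget and countdown that opens the KickOrNot monster widget at zero.
; Clicking the mirror enlarges it, rebuilds its scene-capture render target at higher resolution and may randomly trigger a drift.
; Drifts require grabbing the wheel before a timeout, starting a timeline-driven circular skill check.
; Timers compare wheel angle to the moving zone, counting misses toward placeholder win/lose messages.
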(event `StopRuleNazad`
  ;[0.04977 0.07792 0.15 0.5] Rulling
  (`KismetSystemLibrary.K2_PauseTimerHandle` (`self.RullNazadGoingTimer`)))

(event `BadEndOfRullEvent`
  ; Вылет в кувейт
  (`KismetSystemLibrary.PrintString` "ВЫ УЛЕТЕ В КУВЕЙТ И УМЕРЛИ" true true (struct :`R` 1.0 :`G` 0.03912 :`A` 1.0) 10.0)
  (set `self.IsStartRulling` true)
  (`KismetSystemLibrary.Delay` 0.2)
  (`self.ResetRull`))

(event `StopSkillCheckRulling`
  ; Стоп Скилл чека
  (`self.StopSkillCheck`)
  (`KismetSystemLibrary.K2_PauseTimerHandle` (`self.TImerSkillCheck`))
  (`KismetSystemLibrary.K2_PauseTimerHandle` (`self.TimerCheck`))
  (set `self.CounterOfFails` 0)
  (`self.ResetRull`)
  (set `self.IsStartRulling` false)
  (`self.Stop Rulling`))

(event `StartRuleNazad`
  ;[0.04977 0.07792 0.15 0.5] Rulling
  (if (`KismetSystemLibrary.K2_IsValidTimerHandle` (`self.RullNazadGoingTimer`))
    (`KismetSystemLibrary.K2_UnPauseTimerHandle` (`self.RullNazadGoingTimer`))
    (else
      (bind _returnvalue (`KismetSystemLibrary.K2_SetTimerDelegate` (delegate `RullNazadGo`) 0.01 true))
      (set `self.RullNazadGoingTimer` _returnvalue))))

(event `Stop Rulling`
  ;[0.04977 0.07792 0.15 0.5] Rulling
  (set `self.IsRulling` false)
  (`KismetSystemLibrary.K2_PauseTimerHandle` (`self.TimerRulling`)))

(event `BadEnd`
  ; Вылет в кувейт
  (`KismetSystemLibrary.PrintString` "Ну ты короче не справился с управлением и теперь лежишь" true true (struct :`R` 1.0 :`G` 0.03912 :`A` 1.0) 10.0))

(event `RullNazadGo`
  (bind (_relativerotation_roll _relativerotation_pitch _relativerotation_yaw) (`KismetMathLibrary.BreakRotator` (`SceneComponent.RelativeRotation` (`self.Wheel`))))
  ;[0.04977 0.07792 0.15 0.5] Rulling
  (if (`self.IsRulling`)
    (`self.StopRuleNazad`)
    (else
      (`SceneComponent.K2_SetRelativeRotation` (`self.Wheel`) (`KismetMathLibrary.MakeRotator` _relativerotation_roll (`KismetMathLibrary.FInterpTo` _relativerotation_pitch 0.0 (`GameplayStatics.GetWorldDeltaSeconds`) 1.0) _relativerotation_yaw) false false))))

(event `Start Rulling`
  ;[0.04977 0.07792 0.15 0.5] Rulling
  (set `self.IsRulling` true)
  (if (`KismetSystemLibrary.K2_IsValidTimerHandle` (`self.TimerRulling`))
    (`KismetSystemLibrary.K2_UnPauseTimerHandle` (`self.TimerRulling`))
    (else
      (bind _returnvalue (`KismetSystemLibrary.K2_SetTimerDelegate` (delegate `Move`) 0.01 true))
      (set `self.TimerRulling` _returnvalue))))

(event `GoodEnd`
  ; Вылет в кувейт
  (`KismetSystemLibrary.PrintString` "ЕЕЕЕ  ВЫ КОРОЧЕ КРУТЫЕ И ТД" true true (struct :`R` 0.168277 :`G` 1.0 :`A` 1.0) 10.0))

(event `Move`
  (bind (_locationx _locationy) (`PlayerController.GetMousePosition` (`GameplayStatics.GetPlayerController` 0)))
  (bind (_x _y) (`KismetMathLibrary.BreakVector2D` (`GameplayStatics.ProjectWorldToScreen` (`GameplayStatics.GetPlayerController` 0) (`SceneComponent.K2_GetComponentLocation` (`self.Wheel`)))))
  (bind (_returnvalue_roll _returnvalue_pitch _returnvalue_yaw) (`KismetMathLibrary.BreakRotator` (`KismetMathLibrary.FindLookAtRotation` (`KismetMathLibrary.MakeVector` _x _y) (`KismetMathLibrary.MakeVector` _locationx _locationy 1.0))))
  ;[0.04977 0.07792 0.15 0.5] Rulling
  (`SceneComponent.K2_SetRelativeRotation` (`self.Wheel`) (`KismetMathLibrary.MakeRotator` 0.0 (+ (* _returnvalue_yaw -1.0) -90.0) 90.0) false false))

(event `ResetRull`
  ; Начало Проверки на начало Управления машиной
  (`|ExecutionSequence`
    (:`then_0`
      (set `self.IsStartRulling` false)
      (goto _label :!via `Reset`))
    (:`then_1`
      (set `self.IsStartRulling` false)
      (goto _label_2 :!via `Reset`))))

(event `self.Wheel.OnClicked`
  (params (TouchedComponent :type "PrimitiveComponent Object Reference") (ButtonPressed :type "Key Structure"))
  ;[0.04977 0.07792 0.15 0.5] Rulling
  ;;[0.1912 0.3564 0.4793 0.502] Interact
  (`self.Start Rulling`))

(event `RullDrifting`
  ; Начало Проверки на начало Управления машиной
  (if (not (`self.IsStartRulling`))
    (`|ExecutionSequence`
      (:`then_0`
        (`/Engine/EditorBlueprintResources/StandardMacros.DoOnce` false :!label _label
          (:`Completed`
            (`KismetSystemLibrary.Delay` (`self.TimeToStartRulling`))
            (if (not (`self.IsStartRulling`))
              (`self.BadEndOfRullEvent`)))))
      (:`then_1`
        (if (`self.IsRulling`)
          (`/Engine/EditorBlueprintResources/StandardMacros.DoOnce` false :!label _label_2
            (:`Completed`
              (set `self.IsStartRulling` true)
              (`self.StartSkillCheckRulling`)))
          (else
            (`KismetSystemLibrary.Delay` 0.3)
            (`self.RullDrifting`)))))))

(event `PlaySkill`
  ; Старт Скилл Чека
  (bind (_direction _percent) (`Timeline|SkillCheck` :!via `PlayFromStart` :!label _label_3)
    (:`Update`
      (bind _returnvalue (mod _percent 1.0))
      (if (< _returnvalue 0.0)
        (set `self.Percent` (+ _returnvalue 1.0))
        (else
          (set `self.Percent` _returnvalue))))
    (:`Finished`
      (`self.StopSkillCheckRulling`)
      (if (`self.IsGetOverZone`)
        (`self.BadEnd`)
        (else
          (`self.GoodEnd`)))
      (set `self.IsGetOverZone` false))))

(event `StopSkill`
  ; Старт Скилл Чека
  (goto _label_3 :!via `Stop`))

(event `self.ReceiveTick`
  (params (DeltaSeconds :type "Float (single-precision)")))

(event `self.Wheel.OnReleased`
  (params (TouchedComponent :type "PrimitiveComponent Object Reference") (ButtonReleased :type "Key Structure"))
  ;[0.04977 0.07792 0.15 0.5] Rulling
  ;;[0.1912 0.3564 0.4793 0.502] Interact
  (`self.Stop Rulling` :!label _label_4)
  (if (not (`self.IsEventStarted`))
    (`KismetSystemLibrary.Delay` (`self.RuleNazagTime`))))

(event `StartSkillCheckRulling`
  ; Старт Скилл Чека
  (`KismetSystemLibrary.PrintString` "СКИЛЛ ЧЕЕЕК" true true (struct :`R` 0.1655 :`G` 1.0 :`A` 1.0) 10.0)
  (if (`KismetSystemLibrary.K2_IsValidTimerHandle` (`self.TImerSkillCheck`))
    (`KismetSystemLibrary.K2_UnPauseTimerHandle` (`self.TImerSkillCheck`))
    (`KismetSystemLibrary.K2_UnPauseTimerHandle` (`self.TimerCheck`))
    (`self.PlaySkill`)
    (`self.StartSkillCheck`)
    (else
      (`self.StartSkillCheck`)
      (bind _returnvalue (`KismetSystemLibrary.K2_SetTimerDelegate` (delegate `UpdateSkillCheck`) 0.01 true true))
      (set `self.TImerSkillCheck` _returnvalue)
      (`self.PlaySkill`)
      (bind _returnvalue_2 (`KismetSystemLibrary.K2_SetTimerDelegate` (delegate `UpdateCheck`) 0.1 true true))
      (set `self.TimerCheck` _returnvalue_2))))

(event `Key|LeftMouseButton`
  (params (Key :type "Key Structure"))
  ;[0.04977 0.07792 0.15 0.5] Rulling
  ;;[0.1912 0.3564 0.4793 0.502] Interact
  (:`Released`
    (goto _label_4)))

(event `UpdateSkillCheck`
  (bind (_returnvalue_roll _returnvalue_pitch) (`KismetMathLibrary.BreakRotator` (`SceneComponent.K2_GetComponentRotation` (`self.Arrow`))))
  ; Старт Скилл Чека
  (if (or (== _returnvalue_roll -180.0) (== _returnvalue_roll 180.0))
    (set `self.RuleAngle` (+ 270.0 _returnvalue_pitch))
    (elif (> _returnvalue_pitch 0.0)
      (set `self.RuleAngle` (- 90.0 _returnvalue_pitch))
      (else
        (set `self.RuleAngle` (- 90.0 _returnvalue_pitch)))))
  (set `self.Rule0to1` (/ (`self.RuleAngle`) 360.0))
  (`self.Set Percent` (`self.Percent`)))

(event `RandomEvent`
  ; Сделать шанс/Добавить звук шин
  (if (`KismetMathLibrary.RandomBool`)
    (`self.RullDrifting`)))

(event `self.ReceiveBeginPlay`
  ;[0.5938 0 0 0.5] BeginPlay
  (bind _aswbp_temperature (cast `/Game/UI/WBP_Temperature` (`WidgetComponent.GetWidget` (`self.TemperatureW`))))
  (set `self.TemperatureWBP` _aswbp_temperature)
  (bind _asbp_player (cast `/Game/Blueprints/Player/BP_Player` (`GameplayStatics.GetPlayerPawn` 0)))
  (set `self.Player` _asbp_player)
  (bind _aswbp_circle_progress_bar (cast `/Game/UI/WBP_CircleProgressBar` (`WidgetComponent.GetWidget` (`self.SkillCheckW`))))
  (bind _output_get (set `self.CircleProgressBar` _aswbp_circle_progress_bar))
  (`Widget.SetVisibility` _output_get "Hidden")
  (`self.EnableInput` (`GameplayStatics.GetPlayerController` 0))
  (bind _returnvalue (`|CreateWidget` "/Game/UI/WBP_Timer.WBP_Timer_C" (`GameplayStatics.GetPlayerController` 0)))
  (bind _output_get_2 (set `self.Timer` _returnvalue))
  (`UserWidget.AddToViewport` _output_get_2 0)
  (`self.UpdateMirror`)
  (`KismetSystemLibrary.K2_SetTimerDelegate` (delegate `Sub time`) 1.0 true)
  (`KismetSystemLibrary.DelayUntilNextTick`)
  (set `self.Monster` (`/Game/Blueprints/Characters/BP_Character.Monster?` (`self.Character`))))

(event `self.Mirror.OnClicked`
  (params (TouchedComponent :type "PrimitiveComponent Object Reference") (ButtonPressed :type "Key Structure"))
  ; Update Mirror
  ;;[0.1912 0.3564 0.4793 0.502] Interact
  (`SceneComponent.K2_SetRelativeTransform` (`self.Mirror`) (`self.MirrorBigSize`) false false)
  (set `/Game/Blueprints/Car/BP_BackViewCamera.CameraQualityLevel` 1.0 (`self.LinkedCamera`))
  (`self.UpdateMirror`)
  (`self.RandomEvent`))

(event `StartSkillCheck`
  (`Widget.SetVisibility` (`self.CircleProgressBar`) "HitTestInvisible"))

(event `self.Mirror.OnReleased`
  (params (TouchedComponent :type "PrimitiveComponent Object Reference") (ButtonReleased :type "Key Structure"))
  ; Update Mirror
  ;;[0.1912 0.3564 0.4793 0.502] Interact
  (`SceneComponent.K2_SetRelativeTransform` (`self.Mirror`) (`self.MirrorSize`) false false :!label _label_5)
  (set `/Game/Blueprints/Car/BP_BackViewCamera.CameraQualityLevel` 0.01 (`self.LinkedCamera`))
  (`self.UpdateMirror`))

(event `StopSkillCheck`
  (`Widget.SetVisibility` (`self.CircleProgressBar`) "Hidden"))

(event `Key|LeftMouseButton`
  (params (Key :type "Key Structure"))
  ; Update Mirror
  ;;[0.1912 0.3564 0.4793 0.502] Interact
  (:`Released`
    (goto _label_5)))

(event `Sub time`
  ;[0.5938 0 0 0.5] BeginPlay
  (`/Engine/EditorBlueprintResources/StandardMacros.DecrementInt` (`self.time`)
    (:`  `
      (`/Game/UI/WBP_Timer.SetTimer` (`self.Timer`) (`self.time`))
      (if (== (`self.time`) 0)
        (bind _returnvalue (`|CreateWidget` "/Game/UI/WBP_KickOrNot.WBP_KickOrNot_C" (`GameplayStatics.GetPlayerController` 0)))
        (bind _output_get (set `self.KickOrNot` _returnvalue))
        (`/Game/UI/WBP_KickOrNot.SetMonster` _output_get (`self.Monster`))
        (`UserWidget.AddToViewport` _output_get 0)))))

(event `Set Percent`
  (params (Percent :type "Float (double-precision)"))
  (`/Game/UI/WBP_CircleProgressBar.SetPercent` (`self.CircleProgressBar`) Percent))

(event `UpdateCheck`
  (bind _rule0to1 (`self.Rule0to1`))
  (bind _rule0to1_2 (`self.Rule0to1`))
  ; Чек скилла чека
  (if (>= (- (`self.Percent`) 0.1) 0.0)
    (if (and (<= _rule0to1_2 (`self.Percent`)) (>= _rule0to1_2 (- (`self.Percent`) 0.1)))
      (`KismetSystemLibrary.PrintString` "ЧЕЕЕК" true true (struct :`R` 0.1655 :`G` 1.0 :`A` 1.0) 10.0 :!label _label_6)
      (else
        (`/Engine/EditorBlueprintResources/StandardMacros.IncrementInt` (`self.CounterOfFails`) :!label _label_7
          (:`  `
            (`KismetSystemLibrary.PrintString` "НЕЕЕ ЧЕЕЕК" true true (struct :`R` 1.0 :`G` 0.019557 :`A` 1.0) 10.0)
            (if (>= (`self.CounterOfFails`) (`self.MaxFailAmount`))
              (set `self.IsGetOverZone` true))))))
    (elif (or (<= _rule0to1 (`self.Percent`)) (>= _rule0to1 (- (`self.Percent`) 0.1)))
      (goto _label_6)
      (else
        (goto _label_7)))))

(event `UpdateMirror`
  (bind (_sizex _sizey) (`PlayerController.GetViewportSize` (`GameplayStatics.GetPlayerController` 0)))
  (bind _cameraqualitylevel (`/Game/Blueprints/Car/BP_BackViewCamera.CameraQualityLevel` (`self.LinkedCamera`)))
  ; Update Mirror
  (`/Engine/EditorBlueprintResources/StandardMacros.IsValid` (`self.LinkedCamera`)
    (:`Is Valid`
      (`KismetSystemLibrary.DelayUntilNextTick`)
      (`KismetSystemLibrary.DelayUntilNextTick`)
      (bind _returnvalue (`KismetMaterialLibrary.CreateDynamicMaterialInstance` "/Game/Materials/M_BackViewCam.M_BackViewCam"))
      (bind _output_get (set `self.Mirror_M` _returnvalue))
      (`PrimitiveComponent.SetMaterial` (`self.Mirror`) 0 _output_get)
      (bind _returnvalue_2 (`KismetRenderingLibrary.CreateRenderTarget2D` (`KismetMathLibrary.FTrunc` (* _sizex _cameraqualitylevel)) (`KismetMathLibrary.FTrunc` (* _sizey _cameraqualitylevel)) "RTF_RGBA8"))
      (bind _output_get_2 (set `self.Mirror RT` _returnvalue_2))
      (bind _output_get_3 (set `SceneCaptureComponent2D.TextureTarget` _output_get_2 (`/Game/Blueprints/Car/BP_BackViewCamera.SceneCaptureComponent2D` (`self.LinkedCamera`))))
      (`MaterialInstanceDynamic.SetTextureParameterValue` (`self.Mirror_M`) "Texture" _output_get_3)
      (`MaterialInstanceDynamic.SetScalarParameterValue` (`self.Mirror_M`) "ScreenBrightness" (`self.ScreenBrightness`)))))

(fn `UserConstructionScript`)