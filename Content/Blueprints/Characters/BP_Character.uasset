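; Character Blueprint that randomly decides on BeginPlay whether it is a monster and, if so, periodically flashes a telltale sprite ("priznak", Russian for "sign").
; A looping 15-second timer calls an event that unhides PaperSprite1, waits two seconds, then hides it again.
; Overlap, Tick and the construction script are empty.
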(event `self.ReceiveBeginPlay`
  (set `self.Monster?` (`KismetMathLibrary.RandomBool`))
  (if (`self.Monster?`)
    (`KismetSystemLibrary.K2_SetTimerDelegate` (delegate `Show and Unshow PRIZNAK`) 15.0 true)))

(event `Show and Unshow PRIZNAK`
  (`SceneComponent.SetHiddenInGame` (`self.PaperSprite1`) false false)
  (`KismetSystemLibrary.Delay` 2.0)
  (`SceneComponent.SetHiddenInGame` (`self.PaperSprite1`) true false))

(fn `UserConstructionScript`)