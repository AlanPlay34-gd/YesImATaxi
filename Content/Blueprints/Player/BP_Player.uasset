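; Player Blueprint that tracks money, passenger and suspicion counters and shows the game's ending screens.
; On BeginPlay in L_Game it creates the WBP_Player HUD, which money and suspicion changes then notify.
; Reaching the passenger limit triggers a good or bad ending based on money earned.
; CheckToArrest shows the police ending at the suspicion threshold, while DeathEnd shows the death screen; neither is called within this Blueprint.
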(event `AddSuspCounter`
  (`/Engine/EditorBlueprintResources/StandardMacros.IncrementInt` (`self.SuspicionCounter`)
    (:`  `
      (`/Game/UI/WBP_Player.CheckSusp` (`self.HUD`)))))

(event `AddPassagerCounter`
  (`/Engine/EditorBlueprintResources/StandardMacros.IncrementInt` (`self.PassengersCounter`)
    (:`  `
      (`self.CheckPassagerCount`))))

(event `self.ReceiveBeginPlay`
  (bind _returnvalue (`GameplayStatics.GetCurrentLevelName` true))
  (if (`KismetStringLibrary.EqualEqual_StrStr` _returnvalue "L_Game")
    (`/Engine/EditorBlueprintResources/StandardMacros.IsValid` (`self.HUD`)
      (:`Is Valid`
        _)
      (:`Is Not Valid`
        (bind _returnvalue_2 (`|CreateWidget` "/Game/UI/WBP_Player.WBP_Player_C" (`GameplayStatics.GetPlayerController` 0)))
        (set `self.HUD` _returnvalue_2)))
    (`UserWidget.AddToViewport` (`self.HUD`) 0)
    (`self.UpdateMoney`)))

(event `GoodEnd`
  (bind _returnvalue (`|CreateWidget` "/Game/UI/WBP_GoodEnd.WBP_GoodEnd_C" (`GameplayStatics.GetPlayerController` 0)))
  (`UserWidget.AddToViewport` _returnvalue 0))

(event `AddMoney`
  (params (Amount :type Integer))
  (set `self.MoneyAmount` (+ Amount (`self.MoneyAmount`)))
  (`/Game/UI/WBP_Player.SetMoney` (`self.HUD`) (`self.MoneyAmount`) :!label _label))

(event `EndOfGame`
  (if (>= (`self.MoneyAmount`) 1000)
    (`self.GoodEnd`)
    (else
      (`self.BadEnd`))))

(event `BadEnd`
  (bind _returnvalue (`|CreateWidget` "/Game/UI/WBP_BadEnd.WBP_BadEnd_C" (`GameplayStatics.GetPlayerController` 0)))
  (`UserWidget.AddToViewport` _returnvalue 0))

(event `UpdateMoney`
  (goto _label))

(event `DeathEnd`
  (bind _returnvalue (`|CreateWidget` "/Game/UI/WBP_DeathEnd.WBP_DeathEnd_C" (`GameplayStatics.GetPlayerController` 0)))
  (`UserWidget.AddToViewport` _returnvalue 0))

(event `CheckPassagerCount`
  (if (>= (`self.PassengersCounter`) 7)
    (`self.EndOfGame`)))

(event `CheckToArrest`
  (if (>= (`self.SuspicionCounter`) 3)
    (`self.PoliceEnd`)))

(event `PoliceEnd`
  (bind _returnvalue (`|CreateWidget` "/Game/UI/WBP_PoliceEnd.WBP_PoliceEnd_C" (`GameplayStatics.GetPlayerController` 0)))
  (`UserWidget.AddToViewport` _returnvalue 0))

(fn `UserConstructionScript`)