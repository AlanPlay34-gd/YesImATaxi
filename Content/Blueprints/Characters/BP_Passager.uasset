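; Passenger sprite for a car, configured by a PassagerInfo struct that marks it as human or monster.
; A GetIn timeline slides the flipbook in and reverses it for getting out, while BeginPlay copies the light, temperature and Vnech detection flags.
; InTheCar starts a looping timer that briefly swaps random animations before restoring the base sprite.
; Monsters can also roll an unusual animation, shown only when IsVench is set.
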(event `AnimGetIn`
  (bind (_direction _goloc) (`Timeline|GetIn` :!label _label)
    (:`Update`
      (`SceneComponent.K2_SetRelativeLocation` (`self.PaperFlipbook`) _goloc false false))))

(event `AnimGetOut`
  (goto _label :!via `Reverse`))

(event `self.ReceiveBeginPlay`
  (`self.CheckDetections`))

(event `CheckDetections`
  (bind (_name _ismonstr _hellodialogue _dialogues _patience _chanceforusuaualanim _dialogueforrulelose _sprite _islight _istemperature _isvnech) (break `/Game/Blueprints/Characters/S_Passager` (`self.PassagerInfo`)))
  (if _islight
    (set `self.IsLight` true)
    (else
      (set `self.IsLight` false)))
  (if _istemperature
    (set `self.IsTemperature` true)
    (else
      (set `self.IsTemperature` false)))
  (if _isvnech
    (set `self.IsVench` true)
    (else
      (set `self.IsVench` false))))

(event `InTheCar`
  (bind (_name _ismonstr _hellodialogue _dialogues _patience _chanceforusuaualanim _dialogueforrulelose _sprite) (break `/Game/Blueprints/Characters/S_Passager` (`self.PassagerInfo`)))
  (`PaperFlipbookComponent.SetFlipbook` (`self.PaperFlipbook`) _sprite)
  (if _ismonstr
    (`KismetSystemLibrary.K2_SetTimerDelegate` (delegate `AnimForMonster`) (`self.TimeToAnim`) true)
    (else
      (`KismetSystemLibrary.K2_SetTimerDelegate` (delegate `BasicAnim`) (`self.TimeToAnim`) true))))

(event `AnimForMonster`
  (bind _paperflipbook (`self.PaperFlipbook`))
  (bind (_anim1 _anim2 _unusualanim _duration1 _duration2 _duraion3) (break `/Game/Blueprints/Characters/S_AnimationsForPassager` (`.AnimList_35_40F3DB4D41AD1BA4DC6DA18586142BE0` (break `/Game/Blueprints/Characters/S_Passager` (`self.PassagerInfo`)))))
  (switch `int` (`KismetMathLibrary.RandomIntegerInRange` 0 2)
    (:`0`
      (`PaperFlipbookComponent.SetFlipbook` _paperflipbook _anim1)
      (`KismetSystemLibrary.Delay` _duration1)
      (`PaperFlipbookComponent.SetFlipbook` (`self.PaperFlipbook`) (`.Sprite_41_F53E779F48709A745F85ABB9BD25AF07` (break `/Game/Blueprints/Characters/S_Passager` (`self.PassagerInfo`))) :!label _label_2))
    (:`1`
      (`PaperFlipbookComponent.SetFlipbook` _paperflipbook _anim2)
      (`KismetSystemLibrary.Delay` _duration2)
      (goto _label_2))
    (:`2`
      (if (`self.IsVench`)
        (`PaperFlipbookComponent.SetFlipbook` _paperflipbook _unusualanim)
        (`KismetSystemLibrary.Delay` _duraion3)
        (goto _label_2)))))

(event `BasicAnim`
  (bind _paperflipbook (`self.PaperFlipbook`))
  (bind (_anim1 _anim2 _unusualanim _duration1 _duration2) (break `/Game/Blueprints/Characters/S_AnimationsForPassager` (`.AnimList_35_40F3DB4D41AD1BA4DC6DA18586142BE0` (break `/Game/Blueprints/Characters/S_Passager` (`self.PassagerInfo`)))))
  (if (`KismetMathLibrary.RandomBool`)
    (`PaperFlipbookComponent.SetFlipbook` _paperflipbook _anim1)
    (`KismetSystemLibrary.Delay` _duration1)
    (else
      (`PaperFlipbookComponent.SetFlipbook` _paperflipbook _anim2)
      (`KismetSystemLibrary.Delay` _duration2)))
  (`PaperFlipbookComponent.SetFlipbook` (`self.PaperFlipbook`) (`.Sprite_41_F53E779F48709A745F85ABB9BD25AF07` (break `/Game/Blueprints/Characters/S_Passager` (`self.PassagerInfo`)))))

(fn `UserConstructionScript`)